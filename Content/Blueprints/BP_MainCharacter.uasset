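; BP_MainCharacter is the player character Blueprint, handling crouch visuals and an underwater camera effect.
; Crouch start plays a timeline that squashes the mesh by lerping its Z scale, and crouch end reverses it.
; Camera swimming events keep a count of overlapping fluids, enabling the water post-process on entry and disabling it only when the count drops to zero.
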(event EventStartCameraSwimming
  (Math|Integer|IncrementInt (Variables|Default|GetCameraFluidCollisionsAmount)
    (:%20%20
      (Variables|/Script/Engine.PostProcessComponent|SetbEnabled (Variables|Default|GetWaterPostProcess) true))))

(event EventStopCameraSwimming
  (bind _result (Math|Integer|DecrementInt (Variables|Default|GetCameraFluidCollisionsAmount))
    (:%20%20
      (if (<= _result 0)
        (Variables|Default|SetCameraFluidCollisionsAmount 0)
        (Variables|/Script/Engine.PostProcessComponent|SetbEnabled (Variables|Default|GetWaterPostProcess) false)))))

(event EventOnStartCrouch
  (params (HalfHeightAdjust :type Float%20%28single-precision%29) (ScaledHalfHeightAdjust :type Float%20%28single-precision%29))
  (bind _alpha (Timeline|Crouching Play)
    (:Update
      (Transformation|SetRelativeScale3D (Variables|Character|GetMesh) (Math|Vector|MakeVector 2.0 2.0 (Math|Float|Lerp 7.0 3.5 _alpha))))))

(event EventOnEndCrouch
  (params (HalfHeightAdjust :type Float%20%28single-precision%29) (ScaledHalfHeightAdjust :type Float%20%28single-precision%29))
  (bind _alpha (Timeline|Crouching Reverse)
    (:Update
      (Transformation|SetRelativeScale3D (Variables|Character|GetMesh) (Math|Vector|MakeVector 2.0 2.0 (Math|Float|Lerp 7.0 3.5 _alpha))))))

(fn ConstructionScript)